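; Live Link remap asset that converts MetaHuman CTRL Expressions face curves into ARKit-style blendshapes or VRoid-style Fcl_MTH mouth shapes, selected by 映射方式.
; GetRemappedCurveName renames curves, with a 镜像 flag choosing left/right for most paired shapes.
; RemapCurveElements merges intermediate names using max or average macros and tunes several with clamps and range remaps, including jawOpen-limited mouthClose.
; ARKit-path blink is disabled, noted as moved to the AnimBP.
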(fn `GetRemappedCurveName`
  (params (CurveName :type Name))
  (returns (ReturnValue :type Name))
  (if (`self.映射方式`)
    (switch `name` CurveName
      (:`Default`
        (switch `name` CurveName
          (:`Default`
            (switch `name` CurveName
              (:`Default`
                (return "None"))
              (:`CTRL_expressions_eyeLookUpL`
                ; 眼睛方向
                (`self.镜像反转` :!label _label
                  (:`左`
                    _)
                  (:`左反转`
                    (return "eyeLookUpRight"))
                  (:`右`
                    (return "eyeLookUpRight"))
                  (:`右反转`
                    _))
                (return "eyeLookUpLeft"))
              (:`CTRL_expressions_eyeLookUpR`
                (goto _label :!via `右边`))
              (:`CTRL_expressions_eyeLookDownL`
                (`self.镜像反转` :!label _label_2
                  (:`左`
                    _)
                  (:`左反转`
                    (return "eyeLookDownRight"))
                  (:`右`
                    (return "eyeLookDownRight"))
                  (:`右反转`
                    _))
                (return "eyeLookDownLeft"))
              (:`CTRL_expressions_eyeLookDownR`
                (goto _label_2 :!via `右边`))
              (:`CTRL_expressions_eyeLookRightL`
                (`self.镜像反转` :!label _label_3
                  (:`左`
                    _)
                  (:`左反转`
                    (return "eyeLookInRight"))
                  (:`右`
                    (return "eyeLookInRight"))
                  (:`右反转`
                    _))
                (return "eyeLookInLeft"))
              (:`CTRL_expressions_eyeLookLeftR`
                (goto _label_3 :!via `右边`))
              (:`CTRL_expressions_eyeLookLeftL`
                (`self.镜像反转` :!label _label_4
                  (:`左`
                    _)
                  (:`左反转`
                    (return "eyeLookOutRight"))
                  (:`右`
                    (return "eyeLookOutRight"))
                  (:`右反转`
                    _))
                (return "eyeLookOutLeft"))
              (:`CTRL_expressions_eyeLookRightR`
                (goto _label_4 :!via `右边`))))
          (:`CTRL_expressions_mouthFunnelDL`
            ; 圆唇
            (return "嘴1"))
          (:`CTRL_expressions_mouthFunnelDR`
            (return "嘴2"))
          (:`CTRL_expressions_mouthFunnelUL`
            (return "嘴3"))
          (:`CTRL_expressions_mouthFunnelUR`
            (return "嘴4"))
          (:`CTRL_expressions_mouthLipsPushDL`
            ; 嘬嘴
            (return "亲1"))
          (:`CTRL_expressions_mouthLipsPushDR`
            (return "亲2"))
          (:`CTRL_expressions_mouthLipsPushUL`
            (return "亲3"))
          (:`CTRL_expressions_mouthLipsPushUR`
            (return "亲4"))
          (:`CTRL_expressions_mouthLeft`
            ; 嘴巴横向移动
            (`self.镜像反转` :!label _label_5
              (:`左`
                _)
              (:`左反转`
                (return "嘴向右"))
              (:`右`
                (return "嘴向右"))
              (:`右反转`
                _))
            (return "嘴向左"))
          (:`CTRL_expressions_mouthRight`
            (goto _label_5 :!via `右边`))
          (:`CTRL_expressions_mouthUpperLipRollInL`
            ; 嘴唇
            (`self.镜像反转` :!label _label_6
              (:`左`
                _)
              (:`左反转`
                (return "上唇内卷右"))
              (:`右`
                (return "上唇内卷右"))
              (:`右反转`
                _))
            (return "上唇内卷左"))
          (:`CTRL_expressions_mouthUpperLipRollInR`
            (goto _label_6 :!via `右边`))
          (:`CTRL_expressions_mouthLowerLipRollInL`
            (`self.镜像反转` :!label _label_7
              (:`左`
                _)
              (:`左反转`
                (return "下唇内卷右"))
              (:`右`
                (return "下唇内卷右"))
              (:`右反转`
                _))
            (return "下唇内卷左"))
          (:`CTRL_expressions_mouthLowerLipRollInR`
            (goto _label_7 :!via `右边`))
          (:`CTRL_expressions_mouthUpperLipRollOutL`
            (`self.镜像反转` :!label _label_8
              (:`左`
                _)
              (:`左反转`
                (return "上唇外翻右"))
              (:`右`
                (return "上唇外翻右"))
              (:`右反转`
                _))
            (return "上唇外翻左"))
          (:`CTRL_expressions_mouthUpperLipRollOutR`
            (goto _label_8 :!via `右边`))
          (:`CTRL_expressions_mouthLowerLipRollOutL`
            (`self.镜像反转` :!label _label_9
              (:`左`
                _)
              (:`左反转`
                (return "下唇外翻右"))
              (:`右`
                (return "下唇外翻右"))
              (:`右反转`
                _))
            (return "下唇外翻左"))
          (:`CTRL_expressions_mouthLowerLipRollOutR`
            (goto _label_9 :!via `右边`))
          (:`CTRL_expressions_mouthLipsTogetherDL`
            ; 闭嘴
            (return "闭嘴1"))
          (:`CTRL_expressions_mouthLipsTogetherDR`
            (return "闭嘴2"))
          (:`CTRL_expressions_mouthLipsTogetherUL`
            (return "闭嘴3"))
          (:`CTRL_expressions_mouthLipsTogetherUR`
            (return "闭嘴4"))
          (:`CTRL_expressions_mouthCornerUpL`
            ; 微笑
            (`self.镜像反转` :!label _label_10
              (:`左`
                _)
              (:`左反转`
                (return "微笑右"))
              (:`右`
                (return "微笑右"))
              (:`右反转`
                _))
            (return "微笑左"))
          (:`CTRL_expressions_mouthCornerUpR`
            (goto _label_10 :!via `右边`))
          (:`CTRL_expressions_mouthCornerDepressL`
            ; 嘴角下弯
            (`self.镜像反转` :!label _label_11
              (:`左`
                _)
              (:`左反转`
                (return "mouthFrownRight"))
              (:`右`
                (return "mouthFrownRight"))
              (:`右反转`
                _))
            (return "mouthFrownLeft"))
          (:`CTRL_expressions_mouthCornerDepressR`
            (goto _label_11 :!via `右边`))
          (:`CTRL_expressions_mouthDimpleL`
            ; 酒窝
            (`self.镜像反转` :!label _label_12
              (:`左`
                _)
              (:`左反转`
                (return "mouthDimpleRight"))
              (:`右`
                (return "mouthDimpleRight"))
              (:`右反转`
                _))
            (return "mouthDimpleLeft"))
          (:`CTRL_expressions_mouthDimpleR`
            (goto _label_12 :!via `右边`))
          (:`CTRL_expressions_mouthUpperLipRaiseL`
            ; 上唇上移
            (`self.镜像反转` :!label _label_13
              (:`左`
                _)
              (:`左反转`
                (return "mouthUpperUpRight"))
              (:`右`
                (return "mouthUpperUpRight"))
              (:`右反转`
                _))
            (return "mouthUpperUpLeft"))
          (:`CTRL_expressions_mouthUpperLipRaiseR`
            (goto _label_13 :!via `右边`))
          (:`CTRL_expressions_mouthLowerLipDepressL`
            ; 下唇下移
            (`self.镜像反转` :!label _label_14
              (:`左`
                _)
              (:`左反转`
                (return "mouthLowerDownRight"))
              (:`右`
                (return "mouthLowerDownRight"))
              (:`右反转`
                _))
            (return "mouthLowerDownLeft"))
          (:`CTRL_expressions_mouthLowerLipDepressR`
            (goto _label_14 :!via `右边`))
          (:`CTRL_expressions_mouthLipsPressL`
            ; 抿唇
            (`self.镜像反转` :!label _label_15
              (:`左`
                _)
              (:`左反转`
                (return "mouthPressRight"))
              (:`右`
                (return "mouthPressRight"))
              (:`右反转`
                _))
            (return "mouthPressLeft"))
          (:`CTRL_expressions_mouthLipsPressR`
            (goto _label_15 :!via `右边`))
          (:`CTRL_expressions_mouthCornerWideL`
            ; 抿唇
            (`self.镜像反转` :!label _label_16
              (:`左`
                _)
              (:`左反转`
                (return "mouthStretchRight"))
              (:`右`
                (return "mouthStretchRight"))
              (:`右反转`
                _))
            (return "mouthStretchLeft"))
          (:`CTRL_expressions_mouthCornerWideR`
            (goto _label_16 :!via `右边`))))
      (:`CTRL_expressions_eyeBlinkL`
        ; 眼睛
        (`self.镜像反转` :!enabledstate Disabled :!label _label_17
          (:`左`
            _)
          (:`左反转`
            ;; 眨眼（已转移至动画蓝图）
            (return "右眼闭合"))
          (:`右`
            (return "右眼闭合"))
          (:`右反转`
            _))
        (return "左眼闭合"))
      (:`CTRL_expressions_eyeBlinkR`
        (goto _label_17 :!via `右边`))
      (:`CTRL_expressions_eyeWidenL`
        (`self.镜像反转` :!label _label_18
          (:`左`
            _)
          (:`左反转`
            ;; 瞪眼
            (return "eyeWideRight"))
          (:`右`
            (return "eyeWideRight"))
          (:`右反转`
            _))
        (return "eyeWideLeft"))
      (:`CTRL_expressions_eyeWidenR`
        (goto _label_18 :!via `右边`))
      (:`CTRL_expressions_eyeSquintInnerL`
        (goto _label_20 :!via `右边`))
      (:`CTRL_expressions_eyeCheekRaiseL`
        ;; 眯眼
        ;;; 脸颊抬起
        (`self.镜像反转` :!label _label_19
          (:`左`
            _)
          (:`左反转`
            (return "cheekSquintRight"))
          (:`右`
            (return "cheekSquintRight"))
          (:`右反转`
            _))
        (return "cheekSquintLeft"))
      (:`CTRL_expressions_eyeSquintInnerR`
        (`self.镜像反转` :!label _label_20
          (:`左`
            _)
          (:`左反转`
            (return "左眼眼角"))
          (:`右`
            (return "左眼眼角"))
          (:`右反转`
            _))
        (return "右眼眼角"))
      (:`CTRL_expressions_eyeCheekRaiseR`
        (goto _label_19 :!via `右边`))
      (:`CTRL_expressions_browRaiseInL`
        ; 眉心抬起
        (return "眉心左"))
      (:`CTRL_expressions_browRaiseInR`
        (return "眉心右"))
      (:`CTRL_expressions_browDownL`
        (`self.镜像反转` :!label _label_21
          (:`左`
            _)
          (:`左反转`
            ; 眉下压
            (return "browDownRight"))
          (:`右`
            (return "browDownRight"))
          (:`右反转`
            _))
        (return "browDownLeft"))
      (:`CTRL_expressions_browDownR`
        (goto _label_21 :!via `右边`))
      (:`CTRL_expressions_browRaiseOuterL`
        (`self.镜像反转` :!label _label_22
          (:`左`
            _)
          (:`左反转`
            ; 眉尾抬起
            (return "browOuterUpRight"))
          (:`右`
            (return "browOuterUpRight"))
          (:`右反转`
            _))
        (return "browOuterUpLeft"))
      (:`CTRL_expressions_browRaiseOuterR`
        (goto _label_22 :!via `右边`))
      (:`CTRL_expressions_mouthCheekBlowL`
        ; 脸颊鼓气
        (return "左脸颊鼓气"))
      (:`CTRL_expressions_mouthCheekBlowR`
        (return "右脸颊鼓气"))
      (:`CTRL_expressions_noseWrinkleL`
        (`self.镜像反转` :!label _label_23
          (:`左`
            _)
          (:`左反转`
            ; 鼻翼嗤笑/皱鼻
            (return "noseSneerRight"))
          (:`右`
            (return "noseSneerRight"))
          (:`右反转`
            _))
        (return "noseSneerLeft"))
      (:`CTRL_expressions_noseWrinkleR`
        (goto _label_23 :!via `右边`))
      (:`CTRL_expressions_jawOpen`
        ; 张嘴
        (return "张嘴"))
      (:`CTRL_expressions_jawOpenExtreme`
        (return "张大嘴"))
      (:`CTRL_expressions_jawFwd`
        ; 下巴
        (return "jawForward"))
      (:`CTRL_expressions_jawLeft`
        (`self.镜像反转` :!label _label_24
          (:`左`
            _)
          (:`左反转`
            (return "jawRight"))
          (:`右`
            (return "jawRight"))
          (:`右反转`
            _))
        (return "jawLeft"))
      (:`CTRL_expressions_jawRight`
        (goto _label_24 :!via `右边`))
      (:`CTRL_expressions_tongueOut`
        ; 吐舌（未实现）
        (return "tongueOut")))
    (else
      (switch `name` CurveName
        (:`CTRL_expressions_eyeBlinkL`
          (`self.镜像反转` :!label _label_25
            (:`左`
              _)
            (:`左反转`
              ; 眨眼
              (return "eyeBlinkRight"))
            (:`右`
              (return "eyeBlinkRight"))
            (:`右反转`
              _))
          (return "eyeBlinkLeft"))
        (:`CTRL_expressions_eyeBlinkR`
          (goto _label_25 :!via `右边`))
        (:`CTRL_expressions_jawOpen`
          (return "Fcl_MTH_A"))
        (:`CTRL_expressions_mouthFunnelDL`
          ; O
          (return "o1"))
        (:`CTRL_expressions_mouthFunnelDR`
          (return "o2"))
        (:`CTRL_expressions_mouthFunnelUL`
          (return "o3"))
        (:`CTRL_expressions_mouthFunnelUR`
          (return "o4"))
        (:`CTRL_expressions_mouthPressDL`
          ; U
          (return "u1"))
        (:`CTRL_expressions_mouthPressDR`
          (return "u2"))
        (:`CTRL_expressions_mouthPressUL`
          (return "u3"))
        (:`CTRL_expressions_mouthPressUR`
          (return "u4"))
        (:`CTRL_expressions_mouthLeft`
          ; I
          (return "i1"))
        (:`CTRL_expressions_mouthRight`
          (return "i2"))
        (:`CTRL_expressions_mouthStickyUOUTL`
          ; E
          (return "e1"))
        (:`CTRL_expressions_mouthStickyUOUTR`
          (return "e2"))
        (:`CTRL_expressions_mouthStickyDOUTL`
          (return "e3"))
        (:`CTRL_expressions_mouthStickyDOUTR`
          (return "e4"))
        (:`CTRL_expressions_mouthCornerUpL`
          ; 笑
          (return "笑1"))
        (:`CTRL_expressions_mouthCornerUpR`
          (return "笑2"))
        (:`CTRL_expressions_mouthCornerDepressL`
          ; 生气嘴
          (return "sqz1"))
        (:`CTRL_expressions_mouthCornerDepressR`
          (return "sqz2"))
        (:`CTRL_expressions_mouthLipsPressL`
          (return "sqz3"))
        (:`CTRL_expressions_mouthLipsPressR`
          (return "sqz4"))))))

(fn `RemapCurveElements`
  (params (CurveItems :type "Map of Name to Float (single-precision) (by ref)"))
  (if (`self.映射方式`)
    (`|ExecutionSequence`
      (:`then_0`
        ; 眯眼
        (`self.眯眼` "左眼眼角" "cheekSquintLeft" "eyeSquintLeft" CurveItems))
      (:`then_1`
        (`self.眯眼` "右眼眼角" "cheekSquintRight" "eyeSquintRight" CurveItems))
      (:`then_2`
        ; 眉心
        (`self.取最大值（无需镜像）` "眉心左" "眉心右" "browInnerUp" CurveItems))
      (:`then_3`
        ; 闭眼（已转移至动画蓝图）
        (`self.闭眼` "左眼闭合" CurveItems :!enabledstate Disabled))
      (:`then_4`
        (`self.闭眼` "右眼闭合" CurveItems :!enabledstate Disabled))
      (:`then_5`
        ; 脸颊鼓气
        (`self.取最大值（无需镜像）` "左脸颊鼓气" "右脸颊鼓气" "cheekPuff" CurveItems))
      (:`then_6`
        (`self.闭嘴钳制` "张嘴" "张大嘴" "jawOpen" CurveItems))
      (:`then_7`
        (`self.取最大值（四参数钳制）` "亲1" "亲2" "亲3" "亲4" "mouthPucker" CurveItems))
      (:`then_8`
        (`self.取最大值（四参数）` "嘴1" "嘴2" "嘴3" "嘴4" "mouthFunnel" CurveItems))
      (:`then_9`
        ; 嘴唇内卷
        (`self.取最大值（平滑钳制）` "上唇内卷左" "上唇内卷右" "mouthRollUpper" CurveItems))
      (:`then_10`
        (`self.取最大值（无需镜像）` "下唇内卷左" "下唇内卷右" "mouthRollLower" CurveItems))
      (:`then_11`
        ; 嘴唇外翻
        (`self.取最大值（无需镜像）` "上唇外翻左" "上唇外翻右" "mouthShrugUpper" CurveItems))
      (:`then_12`
        (`self.取最大值（无需镜像）` "下唇外翻左" "下唇外翻右" "mouthShrugLower" CurveItems))
      (:`then_13`
        ; 嘴巴横向移动
        (`self.平滑映射` "嘴向左" "mouthLeft" CurveItems 0.08 0.5 0.0 0.6))
      (:`then_14`
        (`self.平滑映射` "嘴向右" "mouthRight" CurveItems 0.08 0.7 0.0 0.6))
      (:`then_15`
        (`self.闭嘴` CurveItems))
      (:`then_16`
        ; 眉毛下压
        (`self.平滑映射` "browDownLeft" "browDownLeft" CurveItems 0.2 1.0 0.0 1.0))
      (:`then_17`
        (`self.平滑映射` "browDownRight" "browDownRight" CurveItems 0.2 1.0 0.0 1.0))
      (:`then_18`
        ; 微笑
        (`self.平滑映射` "微笑左" "mouthSmileLeft" CurveItems 0.0 0.1 0.0 0.4))
      (:`then_19`
        (`self.平滑映射` "微笑右" "mouthSmileRight" CurveItems 0.0 0.1 0.0 0.4))
      (:`then_20`
        ; 酒窝
        (`self.平滑映射` "mouthDimpleLeft" "mouthDimpleLeft" CurveItems 0.0 0.6 0.0 1.0))
      (:`then_21`
        (`self.平滑映射` "mouthDimpleRight" "mouthDimpleRight" CurveItems 0.0 0.6 0.0 1.0))
      (:`then_23`
        (return)))
    (else
      (`|ExecutionSequence`
        (:`then_0`
          (`self.取最大值（四参数）` "o1" "o2" "o3" "o4" "Fcl_MTH_O" CurveItems))
        (:`then_1`
          (`self.取最大值（四参数）` "u1" "u2" "u3" "u4" "Fcl_MTH_U" CurveItems))
        (:`then_2`
          (`self.平均值` "i1" "i2" "Fcl_MTH_I" CurveItems))
        (:`then_3`
          (`self.取最大值（四参数）` "e1" "e2" "e3" "e4" "Fcl_MTH_E" CurveItems))
        (:`then_4`
          (`self.平均值` "笑1" "笑2" "Fcl_MTH_Fun" CurveItems))
        (:`then_5`
          (`self.取最大值（四参数）` "sqz1" "sqz2" "sqz3" "sqz4" "Fcl_MTH_Angry" CurveItems))
        (:`then_6`
          (return))))))